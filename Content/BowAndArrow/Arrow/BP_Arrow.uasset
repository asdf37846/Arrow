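; BP_Arrow is an arrow actor for the bow and arrow, whose mesh continually orients toward the player's bow.
; On BeginPlay it casts the player character to BP_ThirdPersonCharacter and caches its ChildActor as the bow.
; Each Tick it builds a rotation from the normalized direction to a point slightly above the bow, pointing the mesh's X axis there.
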(event EventBeginPlay
  (bind _asbp_third_person_character (Utilities|Casting|CastToBP_ThirdPersonCharacter (Game|GetPlayerCharacter 0)))
  (Variables|Default|SetBow (Variables|/Game/ThirdPerson/Blueprints/BP_ThirdPersonCharacter.BP_ThirdPersonCharacter_C|GetChildActor _asbp_third_person_character)))

(event Collision|EventActorBeginOverlap
  (params (OtherActor :type Actor%20Object%20Reference)))

(event EventTick
  (params (DeltaSeconds :type Float%20%28single-precision%29))
  (bind _bow (Variables|Default|GetBow))
  (bind _returnvalue (Transformation|GetWorldLocation _bow))
  (bind (_x _y _z) (Math|Vector|BreakVector _returnvalue))
  (Transformation|SetWorldRotation (Variables|Default|GetStaticMesh) (Math|Rotator|MakeRotfromX (Math|Vector|Normalize (- (Math|Vector|MakeVector _x _y (+ _z 2.0)) (Transformation|GetWorldLocation (Variables|Default|GetStaticMesh))))) false false))

(fn ConstructionScript)