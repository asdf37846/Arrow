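; BP_ArrowFly is an arrow projectile that sticks into what it hits and damages Target actors.
; On arrowhead overlap with another actor, it stops its ProjectileMovement, zeroes gravity and attaches to that actor, keeping world transform.
; A successful Target cast subtracts fixed damage directly from its Heath variable, then destroys the arrow after a short delay.
; A failed cast ends execution, so arrows in other actors are not destroyed here.
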(event OnComponentBeginOverlap(ArrowheadCol)
  (params (OverlappedComponent :type Primitive%20Component%20Object%20Reference) (OtherActor :type Actor%20Object%20Reference) (OtherComp :type Primitive%20Component%20Object%20Reference) (OtherBodyIndex :type Integer) (bFromSweep :type Boolean) (SweepResult :type Hit%20Result%20Structure%20%28by%20ref%29))
  (bind _projectilemovement (Variables|Default|GetProjectileMovement))
  (if (!= OtherActor self)
    (Components|Movement|StopMovementImmediately _projectilemovement)
    (Variables|/Script/Engine.ProjectileMovementComponent|SetProjectileGravityScale _projectilemovement 0.0)
    (Transformation|AttachActorToActor OtherActor "None" "KeepWorld" "KeepWorld" "KeepWorld" true)
    ;[1 1 1] Arrow Damage
    (bind _astarget (Utilities|Casting|CastToTarget OtherActor))
    (if (== _astarget OtherActor)
      (Variables|/Game/Test/Target.Target_C|SetHeath _astarget (- (Variables|/Game/Test/Target.Target_C|GetHeath _astarget) 5e+01)))
    (Utilities|FlowControl|Delay 1.0)
    (Actor|DestroyActor)))

(event EventBeginPlay)

(event Collision|EventActorBeginOverlap
  (params (OtherActor :type Actor%20Object%20Reference)))

(event EventTick
  (params (DeltaSeconds :type Float%20%28single-precision%29)))

(fn ConstructionScript)