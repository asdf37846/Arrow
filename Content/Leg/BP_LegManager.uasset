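; BP_LegManager coordinates the left and right legs of its owning BP_ThirdPersonCharacter.
; It collects both leg references on BeginPlay and calls UpdateFoot on each every tick.
; CanLegUnplant permits a leg to lift only while another leg is planted, a check for keeping one foot down.
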(event EventBeginPlay
  (bind _legs (Variables|Default|GetLegs))
  (bind _asbp_third_person_character (Utilities|Casting|CastToBP_ThirdPersonCharacter (Components|GetOwner)))
  (Utilities|Array|Add _legs (Variables|/Game/ThirdPerson/Blueprints/BP_ThirdPersonCharacter.BP_ThirdPersonCharacter_C|GetBP_Leg_Left _asbp_third_person_character))
  (Utilities|Array|Add _legs (Variables|/Game/ThirdPerson/Blueprints/BP_ThirdPersonCharacter.BP_ThirdPersonCharacter_C|GetBP_Leg_Right _asbp_third_person_character)))

(event EventTick
  (params (DeltaSeconds :type Float%20%28single-precision%29))
  (for _array_element (Variables|Default|GetLegs)
    (Default|UpdateFoot _array_element)))

(fn CanLegUnplant
  (params (Leg :type BP%20Leg%20Object%20Reference))
  (for _array_element (Variables|Default|GetLegs)
    (if (and (Variables|/Game/Leg/BP_Leg.BP_Leg_C|GetIsPlanted _array_element) (!= _array_element Leg))
      (return true)))
  (return false))