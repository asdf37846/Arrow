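; BP_Leg computes the procedural foot placement and stepping for one leg, with UpdateFoot driving each update rather than its empty Tick.
; It line-traces along its forward vector for a target, falling back to a vertical trace from the ray's end, then the previous target.
; When the planted foot drifts too far and LegManager permits unplanting, curves drive a timed, arced step from the old position to the continually updated target.
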(event Custom|SetDefaultPosition
  (bind _traceposition (Variables|Default|GetTracePosition))
  (CallFunction|GetFootTargetLocation)
  (Variables|Default|SetPlant%20Start%20Position _traceposition)
  (Variables|Default|SetTargetPosition _traceposition)
  (Variables|Default|SetFootPosition _traceposition))

(event EventBeginPlay
  (Variables|Default|SetFootPosition (Transformation|GetWorldLocation)))

(event EventTick
  (params (DeltaSeconds :type Float%20%28single-precision%29)))

(fn GetFootTargetLocation
  (Utilities|FlowControl|Sequence
    (:then_0
      (Variables|Default|SetRayStart (Transformation|GetWorldLocation)))
    (:then_1
      (Variables|Default|SetRayEnd (+ (Variables|Default|GetRayStart) (* (Math|Vector|GetForwardVector (.Rotation (Math|Transform|BreakTransform (Transformation|GetWorldTransform)))) (Variables|Default|GetRayCastLength)))))
    (:then_2
      (bind _location (Utilities|CastRay (Variables|Default|GetRayStart) (Variables|Default|GetRayEnd))
        (:True
          (Variables|Default|SetTracePosition _location))
        (:False
          (bind _location_2 (Utilities|CastRay (Variables|Default|GetRayEnd) (+ (Variables|Default|GetRayEnd) (Math|Vector|MakeVector 0.0 0.0 (* (Variables|Default|GetRayCastLength) 2.0))))
            (:True
              (Variables|Default|SetTracePosition _location_2))
            (:False
              (Variables|Default|SetTracePosition (Variables|Default|GetTargetPosition)))))))
    (:then_3
      (Variables|Default|SetTargetPosition (Variables|Default|GetTracePosition)))))

(fn CheckforReplant
  (Utilities|FlowControl|Sequence
    (:then_0
      (Variables|Default|SetWant%20to%20Replant (and (Variables|Default|GetIsPlanted) (> (Math|Vector|VectorLength (- (Variables|Default|GetFootPosition) (Variables|Default|GetTargetPosition))) (Variables|Default|GetStopDistance)))))
    (:then_1
      (bind _canunplant (Default|CanLegUnplant (Variables|Default|GetLeg%20Manager) self))
      (Variables|Default|SetDo%20Replant (and (Variables|Default|GetWant%20to%20Replant) _canunplant)))
    (:then_2
      (if (Variables|Default|GetDo%20Replant)
        (Utilities|FlowControl|Sequence
          (:then_0
            (Variables|Default|SetIsPlanted false))
          (:then_1
            (Variables|Default|SetPlant%20Start%20Position (Variables|Default|GetFootPosition)))
          (:then_2
            (Variables|Default|SetTime%20Since%20Unplanted 0.125)))))))

(fn TakeFootstep
  (if (Variables|Default|GetIsPlanted)
    (return)
    (else
      (Utilities|FlowControl|Sequence
        (:then_0
          (Variables|Default|SetPercentage%20Replanted (/ (Variables|Default|GetTime%20Since%20Unplanted) (Variables|Default|GetStopTime))))
        (:then_1
          (Variables|Default|SetFoot%20Position%20No%20Height (Math|Vector|Lerp(Vector) (Variables|Default|GetPlant%20Start%20Position) (Variables|Default|GetTargetPosition) (Math|Curves|GetFloatValue (Variables|Default|GetReplant%20Speed%20Curve) (Variables|Default|GetPercentage%20Replanted)))))
        (:then_2
          (Variables|Default|SetFootPosition (+ (Variables|Default|GetFoot%20Position%20No%20Height) (Math|Vector|MakeVector 0.0 0.0 (* (Math|Curves|GetFloatValue (Variables|Default|GetReplant%20Height%20Curve) (Variables|Default|GetPercentage%20Replanted)) (Variables|Default|GetStop%20Height))))))
        (:then_3
          (bind _output_get (Variables|Default|SetTime%20Since%20Unplanted (+ (Variables|Default|GetTime%20Since%20Unplanted) (Utilities|Time|GetWorldDeltaSeconds))))
          (Variables|Default|SetIsPlanted (>= _output_get (Variables|Default|GetStopTime))))))))

(fn UpdateFoot
  (CallFunction|GetFootTargetLocation)
  (CallFunction|CheckforReplant)
  (CallFunction|TakeFootstep)
  (if (Variables|Debug|GetDebugDraw)
    (CallFunction|Debug)))

(fn Debug
  (Rendering|Debug|DrawDebugSphere (Variables|Default|GetFootPosition) 4.0 12 "(R=0.000000,G=1.000000,B=0.000000,A=1.000000)" 0.0 2.0))